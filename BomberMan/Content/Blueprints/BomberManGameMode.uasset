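; Game mode for a local multiplayer Bomberman game that builds the level and spawns the players on BeginPlay.
; It spawns a FloorData actor with a random grid size and fill percent, then has it create the level.
; It creates the extra local players, then spawns a Bomber_BP for each at the PlayerStart tagged with their player number.
; Each controller possesses its bomber, which then gets its input and color set.
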(event EventBeginPlay
  (CallFunction|CreateLevel)
  (CallFunction|SpawnPlayers))

(event EventTick
  (params (DeltaSeconds :type Float%20%28single-precision%29)))

(fn ConstructionScript)

(fn SpawnPlayers
  (bind _players (Variables|Default|GetPlayers))
  (bind _returnvalue (- _players 1))
  ;[1 1 1] we already have 1 player created so create rest
  (for _index (range 1 _returnvalue)
    (Class|GameplayStatics|CreatePlayer _index))
  ;[1 1 1] Spawn our player and posses and bind our keyboard
  (for _index_2 (range 0 _returnvalue)
    (bind _transform (CallFunction|GetSpawnLocation _index_2))
    (bind _returnvalue_2 (Game|SpawnActorfromClass "/Game/Blueprints/Bomber_BP.Bomber_BP_C" _transform "Undefined" 0 _index_2 0))
    (Pawn|Possess (Game|GetPlayerController _index_2) _returnvalue_2)
    (Class|Bomber|SetInput _returnvalue_2 _index_2)
    (Default|SetPlayerColor _returnvalue_2)))

(fn GetSpawnLocation
  (params (PlayerIndex :type Integer))
  ;[1 1 1] Go throught all the player start and get the transformation for our player index
  (bind _outactors (Actor|GetAllActorsOfClass "/Script/Engine.PlayerStart"))
  (for _array_element _outactors
    (if (Utilities|Enum|Equal(Enum) (Utilities|String|ToString(Name) (Variables|/Script/Engine.PlayerStart|GetPlayerStartTag _array_element)) (Utilities|String|Append "Player" (Utilities|String|ToString(Integer) (+ PlayerIndex 1))))
      (return (Transformation|GetActorTransform _array_element)))))

(fn CreateLevel
  ;[1 1 1] Spawn the floor class and set grid size and the spawn bricks
  (bind _returnvalue (Game|SpawnActorfromClass "/Script/BomberMan.FloorData" (Math|Transform|MakeTransform "0, 0,-2000.000000") "Undefined" 0 0))
  (Class|FloorData|SetGridSize _returnvalue (Math|Random|RandomIntegerinRange 20 40))
  (Class|FloorData|SetFillPercent _returnvalue (Math|Random|RandomFloatinRange 0.3 0.7))
  (Class|FloorData|CreateLevel _returnvalue))