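; Game state for a two-player Bomberman match that runs the round timer and resolves the result.
; Tick counts down from MaxTime, then calls CheckWinLose without zeroing CurrentTime.
; CheckWinLose picks a winner or draw from death flags, comparing scores only if CurrentTime is at or below zero.
; A result shows the EndGame widget, appends scores and status to the SaveData slot, and disables input.
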(event EventBeginPlay
  ;[1 1 1] Set Max Game Time
  (Variables|Default|SetCurrentTime (Variables|Default|GetMaxTime)))

(event EventTick
  (params (DeltaSeconds :type Float%20%28single-precision%29))
  ;[1 1 1] Tick the game time
  (if (> (- (Variables|Default|GetCurrentTime) DeltaSeconds) 0.0)
    (Variables|Default|SetCurrentTime (- (Variables|Default|GetCurrentTime) DeltaSeconds))
    (else
      (CallFunction|CheckWinLose))))

(fn ConstructionScript)

(fn LoadSaveData
  ;[1 1 1] Check if we have save data created or create one
  (bind _returnvalue (SaveGame|DoesSaveGameExist "SaveData"))
  (if _returnvalue
    (bind _returnvalue_2 (SaveGame|LoadGamefromSlot "SaveData"))
    (bind _assave_data (Utilities|Casting|CastToSaveData _returnvalue_2))
    (Variables|Default|SetSaveDataRef _assave_data)
    (else
      (bind _returnvalue_3 (SaveGame|CreateSaveGameObject "/Game/Blueprints/SaveData.SaveData_C"))
      (Variables|Default|SetSaveDataRef _returnvalue_3)))
  (return (Variables|Default|GetSaveDataRef)))

(fn AddtoSaveData
  (params (Status :type String))
  (bind _savedataref (Variables|Default|GetSaveDataRef))
  (LocalVariables|SetStatusText Status)
  ;[1 1 1] Get all the data from the players and store
  (bind _asbomber_bp (Utilities|Casting|CastToBomber_BP (Pawn|GetControlledPawn (Game|GetPlayerController 0))))
  (bind _returnvalue (Class|Bomber|GetScore _asbomber_bp))
  (bind _asbomber_bp_2 (Utilities|Casting|CastToBomber_BP (Pawn|GetControlledPawn (Game|GetPlayerController 1))))
  (bind _returnvalue_2 (Class|Bomber|GetScore _asbomber_bp_2))
  (Utilities|Array|Add (Variables|/Game/Blueprints/SaveData.SaveData_C|GetPlayers _savedataref) "Player1")
  (Utilities|Array|Add (Variables|/Game/Blueprints/SaveData.SaveData_C|GetPlayers _savedataref) "Player2")
  (Utilities|Array|Add (Variables|/Game/Blueprints/SaveData.SaveData_C|GetScore _savedataref) _returnvalue)
  (Utilities|Array|Add (Variables|/Game/Blueprints/SaveData.SaveData_C|GetScore _savedataref) _returnvalue_2)
  (Utilities|Array|Add (Variables|/Game/Blueprints/SaveData.SaveData_C|GetStatus _savedataref) (LocalVariables|GetStatusText))
  (SaveGame|SaveGametoSlot (Variables|Default|GetSaveDataRef) "SaveData"))

(fn CheckWinLose
  ;[1 1 1] Check player dead status
  (bind _asbomber_bp (Utilities|Casting|CastToBomber_BP (Pawn|GetControlledPawn (Game|GetPlayerController 0))))
  (bind _returnvalue (Class|Bomber|IsDead _asbomber_bp))
  (LocalVariables|SetPlayer1Dead _returnvalue)
  (bind _returnvalue_2 (Class|Bomber|GetScore _asbomber_bp))
  (LocalVariables|SetPlayer1Score _returnvalue_2)
  (bind _asbomber_bp_2 (Utilities|Casting|CastToBomber_BP (Pawn|GetControlledPawn (Game|GetPlayerController 1))))
  (bind _returnvalue_3 (Class|Bomber|IsDead _asbomber_bp_2))
  (LocalVariables|SetPlayer2Dead _returnvalue_3)
  (bind _returnvalue_4 (Class|Bomber|GetScore _asbomber_bp_2))
  (LocalVariables|SetPlayer2Score _returnvalue_4)
  ;[1 1 1] If Both player are dead show Draw
  (if (LocalVariables|GetPlayer1Dead)
    (if (LocalVariables|GetPlayer2Dead)
      (LocalVariables|SetTitle "DRAW" :!label _label)
      (else
        ;[1 1 1] If Player 1 is dead
        (LocalVariables|SetTitle "PLAYER 2 WIN" :!label _label_2)))
    ;[1 1 1] Show end game widget
    (Viewport|RemoveAllWidgets :!label _label_3)
    (bind _returnvalue_5 (UserInterface|CreateWidget "/Game/Blueprints/UI/EndGame.EndGame_C"))
    (Variables|/Game/Blueprints/UI/EndGame.EndGame_C|SetTitleText _returnvalue_5 (LocalVariables|GetTitle))
    (UserInterface|Viewport|AddtoViewport _returnvalue_5 0)
    ;[1 1 1] Save data
    (CallFunction|LoadSaveData)
    (CallFunction|AddtoSaveData (LocalVariables|GetTitle))
    ;[1 1 1] Disable all inputs
    (bind _asbomber_bp_3 (Utilities|Casting|CastToBomber_BP (Pawn|GetControlledPawn (Game|GetPlayerController 0))))
    (Input|DisableInput _asbomber_bp_3 0)
    (Utilities|Casting|CastToBomber_BP (Pawn|GetControlledPawn (Game|GetPlayerController 1)))
    (Input|DisableInput 0)
    (else
      ;[1 1 1] If Player 2 is dead
      (if (LocalVariables|GetPlayer2Dead)
        (LocalVariables|SetTitle "PLAYER 1 WIN" :!label _label_4)
        (goto _label_3)
        (else
          ;[1 1 1] If Time is finished then check scores
          (if (<= (Variables|Default|GetCurrentTime) 0.0)
            (if (== (LocalVariables|GetPlayer1Score) (LocalVariables|GetPlayer2Score))
              (goto _label)
              (elif (< (LocalVariables|GetPlayer1Score) (LocalVariables|GetPlayer2Score))
                (goto _label_2)
                (else
                  (goto _label_4))))))))))