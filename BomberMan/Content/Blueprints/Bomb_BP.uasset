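; Bomberman-style bomb actor that disables its collision on spawn and explodes when its countdown in Tick runs out.
; The blast hides the mesh and line-traces along ±X and ±Y to the blast distance, destroying the brick hit or setting ShouldExplode on another bomb.
; That flag alone does not cut a timer short, as ExplodeBomb runs only after expiry.
; The following tick calls AddBombs on the spawner and destroys the actor.
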(event EventBeginPlay
  (Collision|SetActorEnableCollision false))

(event EventTick
  (params (DeltaSeconds :type Float%20%28single-precision%29))
  (bind _output_get (Variables|Default|SetBombTimer (- (Variables|Default|GetBombTimer) DeltaSeconds)))
  (if (<= _output_get 0.0)
    (Variables|Default|SetShouldExplode true)
    (CallFunction|ExplodeBomb)))

(fn ConstructionScript)

(fn CheckCollision
  ;[1 1 1] Calculate Start Point and end point in all 4 direction based on blast distance
  (Variables|Default|SetStartPoint (+ (Transformation|GetWorldLocation (Variables|Default|GetStaticMesh)) "0, 0,50.000000"))
  (bind _returnvalue (Class|Bomb|GetBombBlastDistance self))
  (Utilities|FlowControl|Sequence
    (:then_0
      (Variables|Default|SetEndPoint (+ (Variables|Default|GetStartPoint) (* "1.000000, 0, 0" (Math|Conversions|ToFloat(Integer) _returnvalue)))))
    (:then_1
      (Variables|Default|SetEndPoint (+ (Variables|Default|GetStartPoint) (* "-1.000000, 0, 0" (Math|Conversions|ToFloat(Integer) _returnvalue)))))
    (:then_2
      (Variables|Default|SetEndPoint (+ (Variables|Default|GetStartPoint) (* "0.000000,1.000000,0.000000" (Math|Conversions|ToFloat(Integer) _returnvalue)))))
    (:then_3
      (Variables|Default|SetEndPoint (+ (Variables|Default|GetStartPoint) (* "0.000000,-1.000000, 0" (Math|Conversions|ToFloat(Integer) _returnvalue))))))
  ;[1 1 1] Line Trace in all 4 directions
  (bind _outhit (Class|KismetSystemLibrary|LineTraceSinglebyProfile (Variables|Default|GetStartPoint) (Variables|Default|GetEndPoint) "StaticMesh" false 0 "None" true))
  ;[1 1 1] If its brick then destroy it
  (bind _asbrick_bp (Utilities|Casting|CastToBrick_BP (.HitActor (Collision|BreakHitResult _outhit)))
    (:then
      (Actor|DestroyActor _asbrick_bp))
    (:CastFailed
      ;[1 1 1] if its another bomb then expolode it
      (bind _asbomb_bp (Utilities|Casting|CastToBomb_BP (.HitActor (Collision|BreakHitResult _outhit))))
      (Variables|Bomb_BP_C|SetShouldExplode _asbomb_bp true))))

(fn DestroyBomb
  ;[1 1 1] setvisibility false and check collision in 4 directions
  (Rendering|SetVisibility (Variables|Default|GetStaticMesh) false false)
  (CallFunction|CheckCollision))

(fn ExplodeBomb
  (if (Variables|Default|GetExploded)
    (bind _returnvalue (Class|Bomb|GetSpawnedBY self))
    (Class|Bomber|AddBombs _returnvalue)
    (Actor|DestroyActor)
    (elif (Variables|Default|GetShouldExplode)
      (CallFunction|DestroyBomb)
      (Variables|Default|SetExploded true))))