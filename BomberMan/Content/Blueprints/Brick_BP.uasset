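; Brick actor that can be broken, disappearing from view at once and removing itself from the world after a delay.
; DestroyBrick hides the static mesh and sets the Destroyed flag, ignoring repeat calls; it leaves collision untouched.
; While the flag is set, Tick counts SelfDestroyTime down by delta seconds and destroys the actor when it runs out.
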(event EventBeginPlay)

(event Collision|EventActorBeginOverlap
  (params (OtherActor :type Actor%20Object%20Reference)))

(event EventTick
  (params (DeltaSeconds :type Float%20%28single-precision%29))
  ;[1 1 1] Check if actor has to be destroyed
  (if (Variables|Default|GetDestroyed)
    (bind _output_get (Variables|Default|SetSelfDestroyTime (- (Variables|Default|GetSelfDestroyTime) DeltaSeconds)))
    (if (<= _output_get 0.0)
      (Actor|DestroyActor))))

(fn ConstructionScript)

(fn DestroyBrick
  ;[1 1 1] Set Actor Visiblty false on Destroy
  (if (not (Variables|Default|GetDestroyed))
    (Rendering|SetVisibility (Variables|Default|GetStaticMesh) false false)
    (Variables|Default|SetDestroyed true)))