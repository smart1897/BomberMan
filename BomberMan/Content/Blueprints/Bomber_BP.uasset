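; Bomber player Blueprint that places bombs and tints its body by player.
; PlaceBomb checks the available bomb count, consumes one and spawns a Bomb_BP at the actor's X/Y on zero height, passing it the owner and blast distance.
; SetPlayerColor creates a dynamic material instance on the mesh and sets its BodyColor from PlayerID, covering two players.
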(event EventBeginPlay)

(event Collision|EventActorBeginOverlap
  (params (OtherActor :type Actor%20Object%20Reference)))

(event EventTick
  (params (DeltaSeconds :type Float%20%28single-precision%29)))

(event EventPlaceBomb
  (bind _self self)
  (bind _self_2 self)
  (bind _returnvalue (Transformation|GetActorLocation _self))
  ;[1 1 1] Check if we can place bomb
  (bind _returnvalue_2 (Class|Bomber|GetBombsAvailable))
  (if (> _returnvalue_2 0)
    ;[1 1 1] If Yes than consume one bomb and spawn bomb at player location
    (Class|Bomber|SubtractBombs)
    (bind _returnvalue_3 (Game|SpawnActorfromClass "/Game/Blueprints/Bomb_BP.Bomb_BP_C" (Math|Transform|MakeTransform (Math|Vector|MakeVector (.x _returnvalue) (.y _returnvalue) 0.0)) "Undefined" 0 0))
    ;[1 1 1] Set Bomb properties
    (Class|Bomb|Spawnedby _returnvalue_3 _self_2)
    (bind _returnvalue_4 (Class|Bomber|GetBombDistance _self_2))
    (Class|Bomb|SetBombBlastDistance _returnvalue_3 _returnvalue_4)))

(fn ConstructionScript)

(fn SetPlayerColor
  (bind _mesh (Variables|Character|GetMesh))
  ;[1 1 1] Get Material based on player index and set color
  (bind _returnvalue (Rendering|Material|CreateDynamicMaterialInstance _mesh 0 (Rendering|Material|GetMaterial _mesh 0) :!class /Script/Engine.PrimitiveComponent))
  (switch int (Variables|Default|GetPlayerID)
    (:0
      (Rendering|Material|SetVectorParameterValue _returnvalue "BodyColor" (Utilities|Struct|MakeLinearColor 1.0 1.0 0.0 0.0) :!class /Script/Engine.MaterialInstanceDynamic))
    (:1
      (Rendering|Material|SetVectorParameterValue _returnvalue "BodyColor" (Utilities|Struct|MakeLinearColor 0.0 1.0 1.0 0.0) :!class /Script/Engine.MaterialInstanceDynamic))))